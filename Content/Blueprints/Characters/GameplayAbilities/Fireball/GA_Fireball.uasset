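; Fireball gameplay ability that plays a melee combo montage, then launches a BP_Fireball from the player character's transform.
; Activation commits the ability and triggers the UI cooldown before the montage starts.
; On montage completion or blend out, it spawns the fireball with an outgoing GE_Dash_Damage effect spec and the player as instigator, then ends.
; Interruption or cancellation ends the ability without spawning.
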(event Ability|EventActivateAbility
  (Ability|CommitAbility)
  (CallFunction|DoUICooldown)
  (|PlayMontageandWaitProxy "None" "/Game/Blueprints/Characters/Animation/AM_Shinbi_Melee_Combo_03.AM_Shinbi_Melee_Combo_03" 1.0 "None" true 1.0
    (:OnCompleted
      (bind _characterbase (CallFunction|GetPlayerCharacterandController :!label _label))
      (Game|SpawnActorfromClass "/Game/Blueprints/Characters/GameplayAbilities/Fireball/BP_Fireball.BP_Fireball_C" (Transformation|GetActorTransform _characterbase) "AlwaysSpawn" 0 (Ability|MakeOutgoingGameplayEffectSpec "/Game/Blueprints/Characters/GameplayAbilities/Dash/GE_Dash_Damage.GE_Dash_Damage_C") _characterbase)
      (Ability|EndAbility))
    (:OnBlendOut
      (goto _label))
    (:OnInterrupted
      (Ability|EndAbility :!label _label_2))
    (:OnCancelled
      (goto _label_2))))

(event Ability|EventOnEndAbility
  (params (bWasCancelled :type Boolean))
  (|CallParentFunction bWasCancelled) ; This node is disabled and will not be called.\nDrag off pins to build functionality.
)