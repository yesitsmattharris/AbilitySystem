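; GA_FireBlast is a gameplay ability that pulls nearby characters toward its owner and stuns them.
; It plays the Shinbi fire blast montage and waits for the pull gameplay event.
; The event triggers instant radius targeting through GATargetActorGetAround, then calls PushCharacter on each BP_CharacterBase with an impulse aimed at the owner.
; The ability ends when the montage completes, blends out, or is interrupted or cancelled.
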(event Ability|EventActivateAbility
  (|PlayMontageandWaitProxy "None" "/Game/Blueprints/Characters/Animation/AM_FireBlast_Shinbi.AM_FireBlast_Shinbi" 1.0 "None" true 1.0
    (:then
      (Ability|Tasks|WaitGameplayEvent "(TagName=\"skill.fireBlast.pull\")" 0
        (:EventReceived
          (bind _data (|WaitTargetData :ConfirmationType "Instant" :Class "/Script/AbilitySystemTest.GATargetActorGetAround" :Radius 6e+02 :ReticleClass 0)
            (:ValidData
              (for _array_element (Ability|TargetData|GetActorsfromTargetData _data)
                (bind _asbp_character_base (Utilities|Casting|CastToBP_CharacterBase _array_element))
                (Default|PushCharacter _asbp_character_base (Math|Vector|Normalize (- (Transformation|GetActorLocation (Ability|GetOwningActorfromActorInfo)) (Transformation|GetActorLocation _asbp_character_base))) 1.2e+03 3.0)))))))
    (:OnCompleted
      (Ability|EndAbility :!label _label))
    (:OnBlendOut
      (goto _label))
    (:OnInterrupted
      (goto _label))
    (:OnCancelled
      (goto _label))))

(event Ability|EventOnEndAbility
  (params (bWasCancelled :type Boolean)))