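; Ground Blast gameplay ability: a targeted area attack that damages and knocks characters into the air.
; After a cost check, it plays a targeting montage and waits for user-confirmed target data from a ground-select target actor, while camera control rotation is enabled.
; On confirm it commits, starts the UI cooldown, plays the cast montage, spawns the blast effect, applies damage and pushes targets upward with a stun.
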(event Ability|EventActivateAbility
  (bind _can (CallFunction|IsCostStillAvailable))
  (if _can
    (|PlayMontageandWaitProxy "None" "/Game/Blueprints/Characters/Animation/AM_GroundBlast_Targeting.AM_GroundBlast_Targeting" 1.0 "None" true 1.0
      (:then
        (Utilities|FlowControl|Delay (Variables|/Script/Engine.AnimSequenceBase|GetSequenceLength (Animation|GetCurrentMontage :!class /Script/GameplayAbilities.GameplayAbility)))
        (bind _characterbase (CallFunction|GetPlayerCharacterandController))
        (Default|MakeCameraControlRotation _characterbase true)
        (bind _data (|WaitTargetData :ConfirmationType "UserConfirmed" :Class "/Game/Blueprints/Characters/GameplayAbilities/GroundBlast/BP_GATargetActorGroundSelect.BP_GATargetActorGroundSelect_C" :ReticleClass 0)
          (:ValidData
            (bind _characterbase_2 (CallFunction|GetPlayerCharacterandController))
            (Variables|/Game/Blueprints/Characters/BP_CharacterBase.BP_CharacterBase_C|SetTargeting _characterbase_2 false)
            (Ability|CommitAbility)
            (CallFunction|DoUICooldown)
            (|PlayMontageandWaitProxy "None" "/Game/Blueprints/Characters/Animation/AM_GroundBlast_Cast.AM_GroundBlast_Cast" 1.0 "None" true 1.0
              (:then
                (Effects|SpawnEmitteratLocation "/Game/Blueprints/Characters/GameplayAbilities/GroundBlast/P_GroundBlast.P_GroundBlast" (Class|AbilitySystemBlueprintLibrary|GetTargetDataEndPoint _data (- (Ability|TargetData|GetDataCountfromTargetData _data) 1)))
                (GameplayEffects|ApplyGameplayEffectToTarget _data "/Game/Blueprints/Characters/GameplayAbilities/GroundBlast/GE_GroundBlast_Damage.GE_GroundBlast_Damage_C" 1 1)
                (for _array_element (Ability|TargetData|GetActorsfromTargetData _data)
                  (bind _asbp_character_base (Utilities|Casting|CastToBP_CharacterBase _array_element))
                  (Default|PushCharacter _asbp_character_base "0, 0,1.000000" 5e+02 2.0 "/Game/Blueprints/Characters/Animation/AM_GroundBlastInAir_Shinbi.AM_GroundBlastInAir_Shinbi")
                  (Utilities|FlowControl|Delay 1.0)
                  (bind _characterbase_3 (CallFunction|GetPlayerCharacterandController))
                  (Default|MakeCameraControlRotation _characterbase_3 false)))
              (:OnCompleted
                (Ability|EndAbility :!label _label))
              (:OnBlendOut
                (goto _label))
              (:OnInterrupted
                (goto _label))
              (:OnCancelled
                (goto _label))))
          (:Cancelled
            (Ability|EndAbility)))))
    (else
      (Ability|EndAbility))))

(event Ability|EventOnEndAbility
  (params (bWasCancelled :type Boolean))
  (bind _characterbase (CallFunction|GetPlayerCharacterandController))
  (Default|MakeCameraControlRotation _characterbase false))